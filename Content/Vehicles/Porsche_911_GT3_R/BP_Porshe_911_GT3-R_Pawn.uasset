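; Drivable Porsche 911 GT3 R Chaos vehicle pawn with engine audio and switchable camera views.
; BeginPlay assigns the rear wheel references to the tire emitter variables and caches the Chaos wheeled movement component.
; Tick feeds RevPercent into the engine MetaSound's RPM parameter, while the camera input cycles through chase, interior and hood cameras by index.
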(event Input|EnhancedActionEvents|EnhancedInputActionIA_CameraChange
  (params (ActionValue :type Boolean) (ElapsedSeconds :type Float%20%28double-precision%29) (TriggeredSeconds :type Float%20%28double-precision%29) (InputAction :type Input%20Action%20Object%20Reference :default "/Game/Input/IA_CameraChange.IA_CameraChange"))
  ;[1 1 1] InputAction CameraChange
  (:Triggered
    (Components|Activation|SetActive (Variables|Default|GetCamera_BehindCar) false false)
    (switch int (Variables|Default|GetCamera%20Index)
      (:0
        (Variables|Default|SetCamera%20Index 1)
        (Components|Activation|SetActive (Variables|Default|GetCamera_CarInterior) true false))
      (:1
        (Variables|Default|SetCamera%20Index 2)
        (Components|Activation|SetActive (Variables|Default|GetCamera_Hood) true false))
      (:2
        (Variables|Default|SetCamera%20Index 0)
        (Components|Activation|SetActive (Variables|Default|GetCamera_BehindCar) true false)))))

(event EventBeginPlay
  ;[1 1 1] Event BeginPlay
  (Utilities|FlowControl|Sequence
    (:then_0
      (Variables|Default|SetTireEmitterBackLeft (Variables|Default|GetWheel_Rear_Left)))
    (:then_1
      (Variables|Default|SetTireEmitterBackRight (Variables|Default|GetWheel_Rear_Right)))
    (:then_2
      (bind _aschaos_wheeled_vehicle_movement_component (Utilities|Casting|CastToChaosWheeledVehicleMovementComponent (Variables|Default|GetVehicleMovementComponent)))
      (Variables|Default|SetWheeled%20Vehicle%20Movement%20Component _aschaos_wheeled_vehicle_movement_component))))

(event EventTick
  (params (DeltaSeconds :type Float%20%28single-precision%29))
  ;[1 1 1] Set Engine Audio Rev Percentage
  (Audio|Parameter|SetFloatParameter (Variables|Default|GetMetaSound_Engine) "Engine RPM" (Variables|Default|GetRevPercent) :!class /Script/Engine.AudioComponent))

(fn ConstructionScript)